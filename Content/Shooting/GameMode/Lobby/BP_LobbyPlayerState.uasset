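; Lobby player state that holds a replicated nickname for a player in the shooting game's lobby.
; On BeginPlay it registers itself with the first local controller's lobby HUD, or, if that cast fails, sets a short one-shot timer naming ChangeNickName, a function that takes a nickname parameter.
; ChangeNickName sets the value, and its RepNotify broadcasts the new name through an event dispatcher.
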(event EventBeginPlay
  (bind _asbp_lobby_hud (Utilities|Casting|CastToBP_LobbyHUD (HUD|GetHUD (Game|GetPlayerController 0)))
    (:then
      (Default|BindPlayerState _asbp_lobby_hud self))
    (:CastFailed
      (Utilities|Time|SetTimerbyFunctionName 0 "ChangeNickName" 0.01))))

(fn ConstructionScript)

(fn ChangeNickName
  (params (NickName :type String))
  (Variables|Default|SetNickName NickName))

(fn OnRepNickName
  (Default|CallEventDispatcherChangeNickName (Variables|Default|GetNickName)))