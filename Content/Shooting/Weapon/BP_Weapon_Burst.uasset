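; BP_Weapon_Burst is a child weapon Blueprint that fires a three-shot burst per trigger press.
; On press, EventTrigger resets the shot count, fires immediately and starts a looping timer on DoTrigger, ignoring presses while that timer exists.
; DoTrigger calls the parent's firing logic while CanShoot allows, then clears the timer after the third shot or when shooting is no longer possible.
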(event EventBeginPlay
  (|CallParentFunction) ; This node is disabled and will not be called.\nDrag off pins to build functionality.
)

(event Collision|EventActorBeginOverlap
  (params (OtherActor :type Actor%20Object%20Reference))
  (|CallParentFunction OtherActor) ; This node is disabled and will not be called.\nDrag off pins to build functionality.
)

(event EventTick
  (params (DeltaSeconds :type Float%20%28single-precision%29))
  (|CallParentFunction DeltaSeconds) ; This node is disabled and will not be called.\nDrag off pins to build functionality.
)

(fn ConstructionScript
  (|CallParentFunction))

(fn EventTrigger
  (params (IsPress :type Boolean))
  (if IsPress
    (if (not (Class|KismetSystemLibrary|TimerExists 0 "DoTrigger"))
      (Variables|Default|SetShootCnt 0)
      (CallFunction|DoTrigger)
      (Utilities|Time|SetTimerbyFunctionName 0 "DoTrigger" 0.1 true)
      (return false))))

(fn DoTrigger
  (if (CallFunction|CanShoot)
    (|CallParentFunction)
    (bind _output_get (Variables|Default|SetShootCnt (+ (Variables|Default|GetShootCnt) 1)))
    (if (>= _output_get 3)
      (Utilities|Time|ClearTimerbyFunctionName 0 "DoTrigger"))
    (else
      (Utilities|Time|ClearTimerbyFunctionName 0 "DoTrigger"))))